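; RoadSpline Blueprint that lays out a chain of spline mesh segments, by its name a road, along a spline.
; SetSplinePoints replaces the spline's points with the supplied world-space positions.
; CreateSplineSegments then adds a manually attached, X-forward SplineMeshComponent per adjacent point pair, bending it with world-space locations and tangents.
; Both steps are events to be called, as the construction script is empty.
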(event Custom|CreateSplineSegments
  (bind _spline (Variables|Default|GetSpline))
  (for _index (range 0 (- (Spline|GetNumberOfSplinePoints (Variables|Default|GetSpline)) 2))
    (bind _returnvalue (AddComponent|AddSplineMeshComponent true))
    (SplineMesh|SetForwardAxis _returnvalue "X" true)
    (SplineMesh|SetStartandEnd _returnvalue (Spline|GetLocationatSplinePoint _spline _index "World") (Spline|GetTangentatSplinePoint _spline _index "World") (Spline|GetLocationatSplinePoint _spline (+ _index 1) "World") (Spline|GetTangentatSplinePoint _spline (+ _index 1) "World") true :!class /Script/Engine.SplineMeshComponent)))

(event Custom|SetSplinePoints
  (params (SplinePoints :type Array%20of%20Vectors))
  (Spline|SetSplinePoints (Variables|Default|GetSpline) SplinePoints "World" true))

(fn ConstructionScript)