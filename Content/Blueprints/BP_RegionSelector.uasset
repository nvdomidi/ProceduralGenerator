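; BP_RegionSelector draws a rectangular selection region as a procedural mesh between a start and a moving position.
; Start and end events store their positions, while each move event rebuilds the quad's vertices, triangles and UVs.
; The flat quad sits slightly above the start height, and triangle winding flips with drag direction to keep its facing consistent.
; UVs are normalized to the vertex bounds and inverted on both axes.
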(event EventStartDrawingRegion
  (params (StartPosition :type Vector :default "0, 0, 0"))
  (Variables|Default|SetStartPosition StartPosition))

(event EventMoveDrawingRegion
  (params (MovePosition :type Vector :default "0, 0, 0"))
  (bind _startposition (Variables|Default|GetStartPosition))
  (bind _vertices (CallFunction|CalculateVertices _startposition MovePosition))
  (bind _triangles (CallFunction|CalculateTriangles _startposition MovePosition))
  (bind _uvs (CallFunction|CalculateUVs _vertices))
  (Class|ProceduralMeshComponent|CreateMeshSectionLinearColor (Variables|Default|GetProceduralMesh) 0 _vertices _triangles 0 _uvs 0 0 0 0 0 false))

(event EventEndDrawingRegion
  (params (EndPosition :type Vector :default "0, 0, 0"))
  (Variables|Default|SetEndPosition EndPosition))

(fn ConstructionScript)

(fn CalculateVertices
  (params (StartPos :type Vector) (EndPos :type Vector))
  (bind (_x _y) (Math|Vector|BreakVector EndPos))
  (bind (_x_2 _y_2 _z) (Math|Vector|BreakVector StartPos))
  (bind _returnvalue (+ _z 1e+01))
  (return (Utilities|Array|MakeArray (Math|Vector|MakeVector _x_2 _y_2 _returnvalue) (Math|Vector|MakeVector _x _y_2 _returnvalue) (Math|Vector|MakeVector _x_2 _y _returnvalue) (Math|Vector|MakeVector _x _y _returnvalue))))

(fn CalculateTriangles
  (params (StartPos :type Vector) (EndPos :type Vector))
  (bind (_x _y) (Math|Vector|BreakVector EndPos))
  (bind (_x_2 _y_2) (Math|Vector|BreakVector StartPos))
  (LocalVariables|SetXChange (- _x _x_2))
  (LocalVariables|SetYChange (- _y _y_2))
  (if (!= (Math|Float|Sign(Float) (LocalVariables|GetXChange)) (Math|Float|Sign(Float) (LocalVariables|GetYChange)))
    (return (Utilities|Array|MakeArray (Class|KismetSystemLibrary|MakeLiteralInteger) 1 2 1 3 2))
    (else
      (return (Utilities|Array|MakeArray 1 0 3 0 2 3)))))

(fn CalculateUVs
  (params (Vertices :type Array%20of%20Vectors))
  (for _array_element Vertices
    (Utilities|FlowControl|Sequence
      (:then_0
        (if (> (LocalVariables|GetminX) (.X (Math|Vector|BreakVector _array_element)))
          (LocalVariables|SetminX (.X (Math|Vector|BreakVector _array_element)))))
      (:then_1
        (if (> (LocalVariables|GetminY) (.Y (Math|Vector|BreakVector _array_element)))
          (LocalVariables|SetminY (.Y (Math|Vector|BreakVector _array_element)))))
      (:then_2
        (if (> (.X (Math|Vector|BreakVector _array_element)) (LocalVariables|GetmaxX))
          (LocalVariables|SetmaxX (.X (Math|Vector|BreakVector _array_element)))))
      (:then_3
        (if (> (.Y (Math|Vector|BreakVector _array_element)) (LocalVariables|GetmaxY))
          (LocalVariables|SetmaxY (.Y (Math|Vector|BreakVector _array_element)))))))
  (LocalVariables|SetRangeX (- (LocalVariables|GetmaxX) (LocalVariables|GetminX)))
  (LocalVariables|SetRangeY (- (LocalVariables|GetmaxY) (LocalVariables|GetminY)))
  (for _array_element_2 Vertices
    (if (not (or (< (LocalVariables|GetRangeX) 1e-06) (< (LocalVariables|GetRangeY) 1e-06)))
      (Utilities|Array|Add (LocalVariables|GetVerticeUVs) (Math|Vector2D|MakeVector2D (- 1.0 (/ (- (.X (Math|Vector|BreakVector _array_element_2)) (LocalVariables|GetminX)) (LocalVariables|GetRangeX))) (- 1.0 (/ (- (.Y (Math|Vector|BreakVector _array_element_2)) (LocalVariables|GetminY)) (LocalVariables|GetRangeY)))))))
  (return (LocalVariables|GetVerticeUVs)))