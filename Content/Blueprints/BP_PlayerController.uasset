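; Player controller for a procedural road generation tool that spawns the region selector, road generator and UI widget.
; Left-dragging traces onto the spawn plane to draw a region, with GameState gating input and guide text; holding right mouse turns the camera.
; Widget dispatchers reset the region, apply a chosen or random heatmap to its mesh, or generate curved roads.
; Each road segment starting inside the region bounds becomes a RoadSpline actor.
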(event Custom|ChooseImage
  (Class|RoadGenerator|ChooseImageandApplytoPlane (Variables|Default|GetRoadGenerator) (Variables|/Game/Blueprints/BP_RegionSelector.BP_RegionSelector_C|GetProceduralMesh (Variables|Default|GetRegionSelector)))
  (Variables|Default|SetGameState "NewEnumerator3"))

(event Custom|AllowChooseRegion
  (bind _output_get (Variables|Default|SetGameState "NewEnumerator1"))
  (Default|UpdateGuide (Variables|Default|GetWidgetRoads) _output_get)
  (Class|ProceduralMeshComponent|ClearAllMeshSections (Variables|/Game/Blueprints/BP_RegionSelector.BP_RegionSelector_C|GetProceduralMesh (Variables|Default|GetRegionSelector))))

(event Custom|CreateRoads
  (bind _mousestartpoint (Variables|Default|GetMouseStartPoint))
  (bind _mouseendpoint (Variables|Default|GetMouseEndPoint))
  (bind _regionselector (Variables|Default|GetRegionSelector))
  (bind _returnvalue (> (.y _mousestartpoint) (.y _mouseendpoint)))
  (bind _returnvalue_2 (> (.x _mousestartpoint) (.x _mouseendpoint)))
  (bind _proceduralmesh (Variables|/Game/Blueprints/BP_RegionSelector.BP_RegionSelector_C|GetProceduralMesh _regionselector))
  (if (and (> (Class|ProceduralMeshComponent|GetNumSections _proceduralmesh) 0) (.bSuccess (Utilities|Casting|CastToMaterialInstanceDynamic (Rendering|Material|GetMaterial _proceduralmesh 0))))
    (bind _returnvalue_3 (Class|RoadGenerator|CreateRoads (Variables|Default|GetRoadGenerator) (Variables|Default|GetMouseStartPoint) (Variables|Default|GetMouseEndPoint) "SE_CURVED"))
    (Utilities|FlowControl|Sequence
      (:then_0
        (Variables|Default|SetminX (Math|Float|SelectFloat (.x _mouseendpoint) (.x _mousestartpoint) _returnvalue_2))
        (Variables|Default|SetminY (Math|Float|SelectFloat (.y _mouseendpoint) (.y _mousestartpoint) _returnvalue))
        (Variables|Default|SetmaxX (Math|Float|SelectFloat (.x _mousestartpoint) (.x _mouseendpoint) _returnvalue_2))
        (Variables|Default|SetmaxY (Math|Float|SelectFloat (.y _mousestartpoint) (.y _mouseendpoint) _returnvalue)))
      (:then_1
        (if _returnvalue_3
          (bind (_startpoints _endpoints) (Class|RoadGenerator|RoadSegmentstoStartandEndPoints (Variables|Default|GetRoadGenerator) 4e+01))
          (Variables|Default|SetRoadStartPoints _startpoints)
          (bind _output_get (Variables|Default|SetRoadEndPoints _endpoints))
          (for _index (range 0 (- (Utilities|Array|Length _output_get) 1))
            (if (not (or (or (> (.X (Math|Vector|BreakVector (Utilities|Array|Get(acopy) (Variables|Default|GetRoadStartPoints) _index))) (Variables|Default|GetmaxX)) (> (Variables|Default|GetminX) (.X (Math|Vector|BreakVector (Utilities|Array|Get(acopy) (Variables|Default|GetRoadStartPoints) _index))))) (or (> (.Y (Math|Vector|BreakVector (Utilities|Array|Get(acopy) (Variables|Default|GetRoadStartPoints) _index))) (Variables|Default|GetmaxY)) (> (Variables|Default|GetminY) (.Y (Math|Vector|BreakVector (Utilities|Array|Get(acopy) (Variables|Default|GetRoadStartPoints) _index)))))))
              (bind _returnvalue_4 (Game|SpawnActorfromClass "/Game/Blueprints/RoadSpline.RoadSpline_C" (Math|Transform|MakeTransform "0, 0, 0" "0, 0, 0" "1,1,1") "Undefined" 0 0))
              (Default|SetSplinePoints _returnvalue_4 (Utilities|Array|MakeArray (Utilities|Array|Get(acopy) (Variables|Default|GetRoadStartPoints) _index) (Utilities|Array|Get(acopy) (Variables|Default|GetRoadEndPoints) _index)))
              (Default|CreateSplineSegments _returnvalue_4))))))
    (else
      (Development|PrintString "Cant create roads at this time" true true "(R=0.802083,G=0.000000,B=0.031896,A=1.000000)" 5.0))))

(event Custom|RandomHeatmap
  (Class|RoadGenerator|CreateRandomHeatmapandApplytoPlane (Variables|Default|GetRoadGenerator) (Variables|/Game/Blueprints/BP_RegionSelector.BP_RegionSelector_C|GetProceduralMesh (Variables|Default|GetRegionSelector)) true)
  (Variables|Default|SetGameState "NewEnumerator3"))

(event EventTick
  (params (DeltaSeconds :type Float%20%28single-precision%29))
  (if (or (Utilities|Enum|Equal(Enum) (Variables|Default|GetGameState) "NewEnumerator1") (Utilities|Enum|Equal(Enum) (Variables|Default|GetGameState) "NewEnumerator2"))
    (if (Variables|Default|GetisLeftMousePressed)
      (bind (_hitposition _valid) (CallFunction|GetMouseHitPosition))
      (if _valid
        (bind _output_get (Variables|Default|SetMouseEndPoint _hitposition))
        (Class|BIRegionSelectorInterface|MoveDrawingRegion(Message) (Variables|Default|GetRegionSelector) _output_get)))))

(event EventBeginPlay
  ;[1 1 1] Spawn RegionSelector
  (Development|PrintString "Hello")
  (Input|SetInputModeGameandUI (Game|GetPlayerController 0) 0 "DoNotLock" false)
  (Variables|Default|SetbShowMouseCursor true)
  (bind _returnvalue (Game|SpawnActorfromClass "/Game/Blueprints/BP_RegionSelector.BP_RegionSelector_C" (Math|Transform|MakeTransform "0, 0, 0" "0, 0, 0" "1,1,1") "Undefined" 0 0))
  (Variables|Default|SetRegionSelector _returnvalue)
  (bind _returnvalue_2 (Game|SpawnActorfromClass "/Script/ProcSim.RoadGenerator" (Math|Transform|MakeTransform "0, 0, 0" "0, 0, 0" "1,1,1") "Undefined" 0 0))
  (Variables|Default|SetRoadGenerator _returnvalue_2)
  (bind _returnvalue_3 (UserInterface|CreateWidget "/Game/Blueprints/Widget_CreateRoads.Widget_CreateRoads_C" (Game|GetPlayerController 0)))
  (bind _output_get (Variables|Default|SetWidgetRoads _returnvalue_3))
  (UserInterface|Viewport|AddtoViewport _output_get 0)
  (EventDispatchers|BindEventtoChooseImageDispatcher _output_get (delegate Custom|ChooseImage))
  (EventDispatchers|BindEventtoAllowChooseRegionDispatcher _output_get (delegate Custom|AllowChooseRegion))
  (EventDispatchers|BindEventtoRandomHeatmapDispatcher _output_get (delegate Custom|RandomHeatmap))
  (EventDispatchers|BindEventtoCreateRoadsDispatcher _output_get (delegate Custom|CreateRoads))
  (Default|UpdateGuide (Variables|Default|GetWidgetRoads) (Variables|Default|GetGameState)))

(event Input|AxisEvents|InputAxisLookUp
  (params (AxisValue :type Float%20%28single-precision%29))
  ;[1 1 1] Turn Camera Around
  (if (Variables|Default|GetisRightMousePressed)
    (Pawn|Input|AddControllerPitchInput (Game|Player|GetPlayerPawn 0) AxisValue)))

(event Input|AxisEvents|InputAxisLookRight
  (params (AxisValue :type Float%20%28single-precision%29))
  ;[1 1 1] Turn Camera Around
  (if (Variables|Default|GetisRightMousePressed)
    (Pawn|Input|AddControllerYawInput (Game|Player|GetPlayerPawn 0) AxisValue)))

(event Input|MouseEvents|LeftMouseButton
  (params (Key :type Key%20Structure :default "None"))
  (bind _regionselector (Variables|Default|GetRegionSelector))
  (:Pressed
    (if (or (Utilities|Enum|Equal(Enum) (Variables|Default|GetGameState) "NewEnumerator1") (Utilities|Enum|Equal(Enum) (Variables|Default|GetGameState) "NewEnumerator2"))
      (Variables|Default|SetisLeftMousePressed true)
      (bind (_hitposition _valid) (CallFunction|GetMouseHitPosition))
      (if _valid
        (bind _output_get (Variables|Default|SetMouseStartPoint _hitposition))
        (Class|BIRegionSelectorInterface|StartDrawingRegion(Message) _regionselector _output_get)
        (bind _output_get_2 (Variables|Default|SetGameState "NewEnumerator1"))
        (Default|UpdateGuide (Variables|Default|GetWidgetRoads) _output_get_2))))
  (:Released
    (if (or (Utilities|Enum|Equal(Enum) (Variables|Default|GetGameState) "NewEnumerator1") (Utilities|Enum|Equal(Enum) (Variables|Default|GetGameState) "NewEnumerator2"))
      (Variables|Default|SetisLeftMousePressed false)
      (bind (_hitposition_2 _valid_2) (CallFunction|GetMouseHitPosition))
      (if _valid_2
        (bind _output_get_3 (Variables|Default|SetMouseEndPoint _hitposition_2))
        (Class|BIRegionSelectorInterface|EndDrawingRegion(Message) _regionselector _output_get_3)
        (bind _output_get_4 (Variables|Default|SetGameState "NewEnumerator2"))
        (Default|UpdateGuide (Variables|Default|GetWidgetRoads) _output_get_4)
        (else
          (Class|BIRegionSelectorInterface|EndDrawingRegion(Message) _regionselector (Variables|Default|GetMouseEndPoint))
          (bind _output_get_5 (Variables|Default|SetGameState "NewEnumerator2"))
          (Default|UpdateGuide (Variables|Default|GetWidgetRoads) _output_get_5))))))

(event Input|MouseEvents|RightMouseButton
  (params (Key :type Key%20Structure :default "None"))
  ;[1 1 1] Turn Camera Around
  (:Pressed
    (Variables|Default|SetisRightMousePressed true))
  (:Released
    (Variables|Default|SetisRightMousePressed false)))

(fn ConstructionScript)

(fn GetMouseHitPosition
  (bind _returnvalue (Game|GetPlayerController 0))
  (bind (_worldlocation _worlddirection) (Game|Player|ConvertMouseLocationToWorldSpace _returnvalue))
  (bind _outhit (Collision|LineTraceByChannel _worldlocation (+ _worldlocation (* _worlddirection 2e+08)) "TraceTypeQuery1" false 0 "None"))
  (if (Utilities|IsValid (.HitActor (Collision|BreakHitResult _outhit)))
    (Utilities|Casting|CastToSpawnPlane_BP (.HitActor (Collision|BreakHitResult _outhit))
      (:then
        (return (.Location (Collision|BreakHitResult _outhit)) true))
      (:CastFailed
        _)))
  (return "0, 0, 0" false))